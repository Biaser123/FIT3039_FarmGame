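; BP_ChargingStation is the Blueprint for a charging station that displays charging progress and a repairing quick-time-event prompt.
; On BeginPlay it creates a hidden W_RepairingQTE widget and binds QTE added and removed events to show or hide it.
; Showing the prompt also starts its looping ping-pong animation.
; Every Tick it copies ChargingProgressRatio into its W_Progression widget component and sets the bar's fill to blue.
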(event `self.ReceiveBeginPlay`
  (add `self.QTEAddedEvent` (delegate `AddQTEUI`))
  (add `self.QTERemovedEvent` (delegate `RemoveUI`))
  (bind _returnvalue (`|CreateWidget` "/Game/CardUI/W_RepairingQTE.W_RepairingQTE_C"))
  (set `self.RepairingQTE` _returnvalue)
  (`UserWidget.AddToViewport` _returnvalue 0)
  (set `Widget.Visibility` "Hidden" _returnvalue))

(event `AddQTEUI`
  (bind _repairingqte (`self.RepairingQTE`))
  (set `Widget.Visibility` "Visible" _repairingqte)
  (`UserWidget.PlayAnimation` _repairingqte (`/Game/CardUI/W_RepairingQTE.Animation_QTE` _repairingqte) 0.0 100000 "PingPong" 0.6 false))

(event `RemoveUI`
  (set `Widget.Visibility` "Hidden" (`self.RepairingQTE`)))

(event `self.ReceiveTick`
  (params (DeltaSeconds :type "Float (single-precision)"))
  (bind _asw_progression (cast `/Game/CardUI/W_Progression` (`WidgetComponent.GetUserWidgetObject` (`self.ProgressionWidgetComponent`))))
  (set `/Game/CardUI/W_Progression.CurrentProgressInBar` (`self.ChargingProgressRatio`) _asw_progression)
  (bind _asw_progression_2 (cast `/Game/CardUI/W_Progression` (`WidgetComponent.GetUserWidgetObject` (`self.ProgressionWidgetComponent`))))
  (`ProgressBar.SetFillColorAndOpacity` (`/Game/CardUI/W_Progression.StatusProgressBar` _asw_progression_2) (struct :`R` 0.083688 :`G` 0.242353 :`B` 1.0 :`A` 1.0)))

(fn `UserConstructionScript`)