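; Crop actor that grows a plant chosen from the player's card HUD and shows its care state.
; BeginPlay copies the card's stats and picks the phase-one mesh, then binds crop events to interaction icons, a watering QTE widget and an Ice Pepper harvest card reward.
; Disease events update status-bar mutation icons and Niagara particles.
; Tick feeds growth progress to the progress bar, coloured by Watering or Reaping tag.
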(event `DiseaseIconAdded`
  (params (DiseaseType :type "EPlantMutation Enum" :default "PM_None"))
  (bind _asw_crop_status_bar (cast `/Game/CardUI/W_CropStatusBar` (`WidgetComponent.GetUserWidgetObject` (`self.CropStatusIconComponent`))))
  (`/Game/CardUI/W_CropStatusBar.Add Mutation Icon` _asw_crop_status_bar DiseaseType)
  (`ActorComponent.Activate` (`self.mutationParticles`) false)
  (bind _returnvalue (`self.GetMutationCount`))
  (`NiagaraComponent.SetNiagaraVariableInt` (`self.mutationParticles`) "MutationCount" _returnvalue))

(event `DiseaseIconRemoved`
  (bind _asw_crop_status_bar (cast `/Game/CardUI/W_CropStatusBar` (`WidgetComponent.GetUserWidgetObject` (`self.CropStatusIconComponent`))))
  (`/Game/CardUI/W_CropStatusBar.RemoveMutation Icon` _asw_crop_status_bar)
  (`NiagaraComponent.SetNiagaraVariableBool` (`self.mutationParticles`) "Kill" true)
  (`ActorComponent.Deactivate` (`self.mutationParticles`)))

(event `GerFuelCard`
  (bind _foundwidgets (`WidgetBlueprintLibrary.GetAllWidgetsOfClass` "/Game/CardUI/W_cardHUD.W_cardHUD_C"))
  (`/Game/CardUI/W_cardHUD.AddCardToUI` _foundwidgets "6"))

(event `HarvestIconShown`
  ;[1 1 1] QTE and Icon Shown
  (bind _asw_crops_interaction_icon (cast `/Game/CardUI/W_CropsInteractionIcon` (`WidgetComponent.GetUserWidgetObject` (`self.WaitingForInteractingIconComponent`))))
  (`Image.SetBrushFromTexture` (`/Game/CardUI/W_CropsInteractionIcon.IconImage` _asw_crops_interaction_icon) "/Game/Textures/UI/HavestingIcon.HavestingIcon" false))

(event `WaterIconShown`
  ;[1 1 1] QTE and Icon Shown
  (bind _asw_crops_interaction_icon (cast `/Game/CardUI/W_CropsInteractionIcon` (`WidgetComponent.GetUserWidgetObject` (`self.WaitingForInteractingIconComponent`))))
  (`Image.SetBrushFromTexture` (`/Game/CardUI/W_CropsInteractionIcon.IconImage` _asw_crops_interaction_icon) "/Game/Textures/UI/WateringIcon.WateringIcon" false))

(event `AddQTEUI`
  (bind _waterqte (`self.WaterQTE`))
  ;[1 1 1] QTE add/Remove
  (set `Widget.Visibility` "Visible" _waterqte)
  (`UserWidget.PlayAnimation` _waterqte (`/Game/CardUI/W_WateringQTE.Animation_QTE` _waterqte) 0.0 1 "Forward" 1.0 false))

(event `RemoveUI`
  ;[1 1 1] QTE add/Remove
  (set `Widget.Visibility` "Hidden" (`self.WaterQTE`)))

(event `self.ReceiveBeginPlay`
  (bind _cropmesh (`self.Cropmesh`))
  (bind _asw_crops_interaction_icon (cast `/Game/CardUI/W_CropsInteractionIcon` (`WidgetComponent.GetUserWidgetObject` (`self.WaitingForInteractingIconComponent`))))
  (`Image.SetBrushFromTexture` (`/Game/CardUI/W_CropsInteractionIcon.IconImage` _asw_crops_interaction_icon) "/Game/Textures/UI/SeedingIcon.SeedingIcon" false)
  ;[1 1 1] Set Info
  (bind _foundwidgets (`WidgetBlueprintLibrary.GetAllWidgetsOfClass` "/Game/CardUI/W_cardHUD.W_cardHUD_C"))
  (for _array_element _foundwidgets
    (bind (_rowname _cardname _cardtype _carddescription _card_image _card_background _cardprice _cardnum _growtime _diseasesmayget _oxygenvalue _temperaturevalue) (break `CardData` (`/Game/CardUI/W_cardhand.Card Info pass for crop` (`/Game/CardUI/W_cardHUD.W_cardhand` _array_element))))
    (bind _output_get (set `self.RowName` _rowname))
    (set `self.GrowTime` _growtime)
    (set `self.OxygenValue` _oxygenvalue)
    (set `self.TemperatureValue` _temperaturevalue)
    (set `self.MutationProbabilities` _diseasesmayget)
    (bind _output_get_2 (set `self.Price` _cardprice))
    (set `self.OriginalPrice` _output_get_2)
    (switch `name` _output_get
      (:`5`
        (`SkeletalMeshComponent.SetSkeletalMeshAsset` (`self.Cropmesh`) "/Game/Models/Plants/SM_Torutree_Phase1.SM_Torutree_Phase1"))
      (:`1`
        (`SkeletalMeshComponent.SetSkeletalMeshAsset` _cropmesh "/Game/Models/Plants/SM_IcePepper_Phase1.SM_IcePepper_Phase1"))
      (:`2`
        (`SkeletalMeshComponent.SetSkeletalMeshAsset` (`self.Cropmesh`) "/Game/Models/Plants/SM_Cactopus_Phase1.SM_Cactopus_Phase1"))
      (:`3`
        (`SkeletalMeshComponent.SetSkeletalMeshAsset` _cropmesh "/Game/Models/Plants/SM_StarPlant_Phase1.SM_StarPlant_Phase1")))
    ;[1 1 1] QTE add/Remove
    (add `self.QTEAdded` (delegate `AddQTEUI`))
    (add `self.QTERemoved` (delegate `RemoveUI`))
    ;[1 1 1] QTE and Icon Shown
    (add `self.WaterIconEvent` (delegate `WaterIconShown`))
    (add `self.HarvestingIconEvent` (delegate `HarvestIconShown`))
    (bind _returnvalue (`|CreateWidget` "/Game/CardUI/W_WateringQTE.W_WateringQTE_C"))
    (set `self.WaterQTE` _returnvalue)
    (`UserWidget.AddToViewport` _returnvalue 0)
    (set `Widget.Visibility` "Hidden" _returnvalue)
    (add `self.IcePepperHarvestMaterialEvent` (delegate `GerFuelCard`))
    (add `self.DiseaseAdded` (delegate `DiseaseIconAdded`))
    (add `self.DiseaseRemoved` (delegate `DiseaseIconRemoved`))))

(event `self.ReceiveTick`
  (params (DeltaSeconds :type "Float (single-precision)"))
  (bind _asw_progression (cast `/Game/CardUI/W_Progression` (`WidgetComponent.GetUserWidgetObject` (`self.ProgressionWidgetComponent`))))
  (set `/Game/CardUI/W_Progression.CurrentProgressInBar` (`self.CropProgressRatio`) _asw_progression)
  (for _array_element (`self.Tags`)
    (switch `name` _array_element
      (:`Watering`
        (bind _asw_progression_2 (cast `/Game/CardUI/W_Progression` (`WidgetComponent.GetUserWidgetObject` (`self.ProgressionWidgetComponent`))))
        (bind _statusprogressbar (`/Game/CardUI/W_Progression.StatusProgressBar` _asw_progression_2))
        (`ProgressBar.SetFillColorAndOpacity` _statusprogressbar (struct :`G` 0.163797 :`B` 1.0 :`A` 1.0)))
      (:`Reaping`
        (`ProgressBar.SetFillColorAndOpacity` _statusprogressbar (struct :`R` 0.043203 :`G` 0.267361 :`A` 1.0))))))

(fn `ProgressionCompleteForUI`
  (cast `/Game/CardUI/W_Progression` (`WidgetComponent.GetUserWidgetObject` (`self.ProgressionWidgetComponent`)))
  (set `self.CropProgressRatio` 0.0))

(fn `UserConstructionScript`)