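; 3D printer actor that displays pet progress on a W_Progression bar in its widget component.
; Every Tick, it finds all BP_GridMap actors and copies each one's PetProgressRatio into the widget, so the last one found wins.
; The same loop re-applies a purple fill color to the status bar, and the Blueprint has no other active logic.
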(event `self.ReceiveTick`
  (params (DeltaSeconds :type "Float (single-precision)"))
  (bind _asw_progression (cast `/Game/CardUI/W_Progression` (`WidgetComponent.GetUserWidgetObject` (`self.ProgressionWidgetComponent`))))
  (bind _outactors (`GameplayStatics.GetAllActorsOfClass` "/Game/Blueprints/BP_GridMap.BP_GridMap_C"))
  (for _array_element _outactors
    (set `/Game/CardUI/W_Progression.CurrentProgressInBar` (`GridMap.PetProgressRatio` _array_element) _asw_progression)
    (bind _asw_progression_2 (cast `/Game/CardUI/W_Progression` (`WidgetComponent.GetUserWidgetObject` (`self.ProgressionWidgetComponent`))))
    (`ProgressBar.SetFillColorAndOpacity` (`/Game/CardUI/W_Progression.StatusProgressBar` _asw_progression_2) (struct :`R` 0.544367 :`G` 0.268275 :`B` 1.0 :`A` 1.0))))

(fn `UserConstructionScript`)