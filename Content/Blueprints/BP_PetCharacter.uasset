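; Pet character that, on BeginPlay, becomes an octopus, seeding robot or harvesting robot based on the selected card.
; It reads the card's row from the W_cardHUD widget, then sets the mesh, looping animation and PetSkills.
; Each type also sets RequiredTag on its PetAIController (Watering, Seeding or Reaping) and copies the card's OxygenValue.
; Unmatched rows only set the Default skill.
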(event `self.ReceiveBeginPlay`
  (bind _mesh (`self.Mesh`))
  (bind _foundwidgets (`WidgetBlueprintLibrary.GetAllWidgetsOfClass` "/Game/CardUI/W_cardHUD.W_cardHUD_C"))
  (for _array_element _foundwidgets
    (bind (_rowname _cardname _cardtype _carddescription _card_image _card_background _cardprice _cardnum _growtime _diseasesmayget _oxygenvalue) (break `CardData` (`/Game/CardUI/W_cardhand.Card Info Pass for pet` (`/Game/CardUI/W_cardHUD.W_cardhand` _array_element))))
    ;[1 1 1] 4 is octopus, 8 is seeding robot, 9 is harvesting robot
    (switch `name` _rowname
      (:`Default`
        (set `self.PetSkills` "Default"))
      (:`4`
        (`SkeletalMeshComponent.SetSkeletalMeshAsset` _mesh "/Game/Models/Characters/OctopusRigged.OctopusRigged")
        (`SceneComponent.K2_SetRelativeLocationAndRotation` (`self.Mesh`) (0.0 0.0 -70.0) (struct :`Yaw` 270.0) false false)
        (`SceneComponent.SetRelativeScale3D` (`self.Mesh`) (1.0 1.0 1.2))
        (`SkeletalMeshComponent.PlayAnimation` (`self.Mesh`) "/Game/Animation/OctopusAnimationfbx__1_.OctopusAnimationfbx__1_" true)
        (set `self.PetSkills` "Watering")
        (bind _aspet_aicontroller (cast `PetAIController` (`self.GetController`)))
        (set `PetAIController.RequiredTag` "Watering" _aspet_aicontroller)
        (set `self.OxygenValue` _oxygenvalue :!label _label))
      (:`8`
        (`SkeletalMeshComponent.SetSkeletalMeshAsset` _mesh "/Game/Models/Characters/SM_SeedingRobot.SM_SeedingRobot")
        (`SkeletalMeshComponent.PlayAnimation` (`self.Mesh`) "/Game/Animation/AS_SeedingRobot.AS_SeedingRobot" true)
        (set `self.PetSkills` "Seeding")
        (bind _aspet_aicontroller_2 (cast `PetAIController` (`self.GetController`)))
        (set `PetAIController.RequiredTag` "Seeding" _aspet_aicontroller_2)
        (goto _label))
      (:`9`
        (`SkeletalMeshComponent.SetSkeletalMeshAsset` _mesh "/Game/Models/Characters/SM_HarvestingRobot.SM_HarvestingRobot")
        (`SkeletalMeshComponent.PlayAnimation` (`self.Mesh`) "/Game/Animation/AS_HarvestingRobot.AS_HarvestingRobot" true)
        (set `self.PetSkills` "Harvesting")
        (bind _aspet_aicontroller_3 (cast `PetAIController` (`self.GetController`)))
        (set `PetAIController.RequiredTag` "Reaping" _aspet_aicontroller_3)
        (goto _label)))))

(fn `UserConstructionScript`)